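; BP_Porta is an interactive door that the player opens and closes with the interact action (E key).
; The Box_Door overlap registers the door as the character's LastInteractObj and enables interaction, and leaving the box disables it.
; When enabled, Interact uses a FlipFlop to alternately play and reverse a timeline that drives SMDoor's relative yaw.
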(event `self.Box_Door.OnComponentBeginOverlap`
  (params (OverlappedComponent :type "PrimitiveComponent Object Reference") (OtherActor :type "Actor Object Reference") (OtherComp :type "PrimitiveComponent Object Reference") (OtherBodyIndex :type Integer) (bFromSweep :type Boolean) (SweepResult :type "HitResult Structure (by ref)"))
  ;[1 1 1] Door Outside
  (bind _asbp_master_character (cast `/Game/BP/Gameplay/BP_Master_Character` OtherActor))
  (set `/Game/BP/Gameplay/BP_Master_Character.Last_Interact_Obj` self _asbp_master_character)
  (set `self.Can_Interact?` true))

(event `self.Box_Door.OnComponentEndOverlap`
  (params (OverlappedComponent :type "PrimitiveComponent Object Reference") (OtherActor :type "Actor Object Reference") (OtherComp :type "PrimitiveComponent Object Reference") (OtherBodyIndex :type Integer))
  ;[1 1 1] Door Outside
  (cast `/Game/BP/Gameplay/BP_Master_Character` OtherActor)
  (set `self.Can_Interact?` false))

(event `/Game/Coletaveis_e_Interativos/BP_Interact_interface.Interact`
  ;[1 1 1] Key E to Open and Close
  (if (`self.Can_Interact?`)
    (`/Engine/EditorBlueprintResources/StandardMacros.FlipFlop`
      (:`A`
        (bind (_direction _door_open_door_close) (`Timeline|Door Open/Door Close` :!label _label)
          (:`Update`
            (`SceneComponent.K2_SetRelativeRotation` (`self.SM_Door`) (`KismetMathLibrary.MakeRotator` 0.0 0.0 _door_open_door_close) false false))))
      (:`B`
        (goto _label :!via `Reverse`)))))

(fn `UserConstructionScript`)