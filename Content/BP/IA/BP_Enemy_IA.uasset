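; BP_Enemy_IA is an enemy Blueprint that damages the player through an AttackBox.
; The Ataque event checks whether the player overlaps the box, then after a short delay calls Damage on BP_Master_Character.
; Separately, any actor that begins overlapping the box receives ApplyDamage.
; The Dano function is an empty stub, with disconnected health-bar nodes left unused.
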(event `Ataque`
  (bind _returnvalue (`GameplayStatics.GetPlayerCharacter` 0))
  (if (`PrimitiveComponent.IsOverlappingActor` (`self.AttackBox`) _returnvalue)
    (bind _asbp_master_character (cast `/Game/BP/Gameplay/BP_Master_Character` _returnvalue))
    (`KismetSystemLibrary.Delay` 0.3)
    (`/Game/BP/Gameplay/BP_Master_Character.Damage` _asbp_master_character 10.0)))

(event `self.AttackBox.OnComponentBeginOverlap`
  (params (OverlappedComponent :type "PrimitiveComponent Object Reference") (OtherActor :type "Actor Object Reference") (OtherComp :type "PrimitiveComponent Object Reference") (OtherBodyIndex :type Integer) (bFromSweep :type Boolean) (SweepResult :type "HitResult Structure (by ref)"))
  (`GameplayStatics.ApplyDamage` OtherActor 10.0))

(fn `Dano`
  (params (Dam :type "Float (double-precision)")))

(fn `UserConstructionScript`)