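; BP_Coletavel is a collectible item actor that the third-person character can pick up by interacting.
; Sphere overlap enables interaction, registers it as the character's LastInteractObj and sets a look-at target; leaving disables both interaction and look-at.
; Interact calls the empty Body event, destroys the actor and prints a hard-coded stick pickup message.
; The construction script looks up a DataTable row, with row name None, to set Item and its mesh.
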(event `Body`)

(event `/Game/BP/Coletaveis_e_Interativos/BP_Interact_interface.Interact`
  ;[1 1 1] Interact Event
  (if (`self.Can_Interact?`)
    (`self.Body`)
    (`self.K2_DestroyActor`)
    (`KismetSystemLibrary.PrintString` "1x Stick")))

(event `self.Sphere.OnComponentBeginOverlap`
  (params (OverlappedComponent :type "PrimitiveComponent Object Reference") (OtherActor :type "Actor Object Reference") (OtherComp :type "PrimitiveComponent Object Reference") (OtherBodyIndex :type Integer) (bFromSweep :type Boolean) (SweepResult :type "HitResult Structure (by ref)"))
  ;[1 1 1] Can or Not Can Interact
  (bind _asbp_third_person_character (cast `/Game/ThirdPerson/Blueprints/BP_ThirdPersonCharacter` OtherActor))
  (set `/Game/ThirdPerson/Blueprints/BP_ThirdPersonCharacter.Last_Interact_Obj` self _asbp_third_person_character)
  (set `self.Can_Interact?` true)
  ;[1 1 1] Look it
  (set `/Game/ThirdPerson/Blueprints/BP_ThirdPersonCharacter.IsLookAt` true _asbp_third_person_character)
  (set `/Game/ThirdPerson/Blueprints/BP_ThirdPersonCharacter.LookAtPosition` (`self.K2_GetActorLocation`) _asbp_third_person_character))

(event `self.Sphere.OnComponentEndOverlap`
  (params (OverlappedComponent :type "PrimitiveComponent Object Reference") (OtherActor :type "Actor Object Reference") (OtherComp :type "PrimitiveComponent Object Reference") (OtherBodyIndex :type Integer))
  ;[1 1 1] Can or Not Can Interact
  (bind _asbp_third_person_character (cast `/Game/ThirdPerson/Blueprints/BP_ThirdPersonCharacter` OtherActor))
  (set `self.Can_Interact?` false)
  ;[1 1 1] Look it
  (set `/Game/ThirdPerson/Blueprints/BP_ThirdPersonCharacter.IsLookAt` false _asbp_third_person_character))

(fn `UserConstructionScript`
  (locals (NewLocalVar :type Name :default "Stick"))
  (bind _returnvalue (`|GetDataTableRow` (`.DataTable` (break `DataTableRowHandle` (`self.Data Table Row Handle`))))
    (:`then`
      (bind _output_get (set `self.Item` _returnvalue))
      (`StaticMeshComponent.SetStaticMesh` (`self.SM_xflicih_tier_2`) (`.Mesh_13_AD8EBFA348327AE6E81FAFB76BCF8BFB` (break `/Game/BP/Coletaveis_e_Interativos/Item_Struct` _output_get))))))